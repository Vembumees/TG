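; Test actor that fakes a 2D light with a procedural mesh cut off by surrounding geometry.
; Each Tick it sweeps Visibility line traces in a pitch circle and builds a triangle fan from the hit or end points, with distance mapped into UV.x for falloff.
; The mesh section and dynamic material are created once, then vertices and UVs update in place.
; A delayed check pushes LightColor changes to the material, and construction sizes a collision sphere to LightDistance.
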(event `self.ReceiveBeginPlay`
  (set `self.lineTraceAngle` (/ 360.0 (`KismetMathLibrary.Conv_IntToDouble` (`self.polygon`))))
  (set `self.originalColor` (`self.lightColor`)))

(event `self.ReceiveTick`
  (params (DeltaSeconds :type "Float (single-precision)"))
  (bind _returnvalue (`self.K2_GetActorLocation`))
  (bind _returnvalue_2 (`self.K2_GetActorLocation`))
  (bind _uvs (`self.UVs`))
  (bind _verts (`self.Verts`))
  (`|ExecutionSequence`
    (:`then_0`
      (`KismetArrayLibrary.Array_Clear` _uvs)
      (`KismetArrayLibrary.Array_Clear` (`self.Triangles`))
      (`KismetArrayLibrary.Array_Clear` _verts)
      (`KismetArrayLibrary.Array_Add` _verts)
      (`KismetArrayLibrary.Array_Add` _uvs)
      (set `self.endVector` (`KismetMathLibrary.MakeVector` (`self.LightDistance`)))
      (for _ (range (+ (`self.polygon`) 1))
        (bind (_outhit _returnvalue_3) (`KismetSystemLibrary.LineTraceSingle` :`Start` _returnvalue_2 :`End` (+ _returnvalue_2 (`self.endVector`)) :`TraceChannel` "TraceTypeQuery1" :`bIgnoreSelf` false))
        (set `self.bLineTraceReturn` _returnvalue_3)
        (bind (_bblockinghit _binitialoverlap _time _distance _location _impactpoint _normal _impactnormal _physmat _hitactor _hitcomponent _hitbonename _hititem _faceindex _tracestart _traceend) (`GameplayStatics.BreakHitResult` _outhit))
        (set `self.traceLoc` (- _location _returnvalue))
        (set `self.TraceEnd` (- _traceend _returnvalue))
        (set `self.endVector` (`KismetMathLibrary.GreaterGreater_VectorRotator` (`self.endVector`) (`KismetMathLibrary.MakeRotator` 0.0 (`self.lineTraceAngle`))))
        (if (`self.bLineTraceReturn`)
          (`KismetArrayLibrary.Array_Add` (`self.Verts`) (`self.traceLoc`))
          (`KismetArrayLibrary.Array_Add` (`self.UVs`) (`KismetMathLibrary.MakeVector2D` (`KismetMathLibrary.MapRangeClamped` (`KismetMathLibrary.VSize` (`self.traceLoc`)) 0.0 (`self.LightDistance`))))
          (else
            (`KismetArrayLibrary.Array_Add` (`self.Verts`) (`self.TraceEnd`))
            (`KismetArrayLibrary.Array_Add` (`self.UVs`) (1.0 0.0)))))
      (set `self.triangleOffset` 1)
      (for _ (range (+ (- (`KismetArrayLibrary.Array_Length` (`self.Verts`)) 3) 1))
        (`KismetArrayLibrary.Array_Add` (`self.Triangles`))
        (for _index (range 2)
          (`KismetArrayLibrary.Array_Add` (`self.Triangles`) (+ _index (`self.triangleOffset`))))
        (`/Engine/EditorBlueprintResources/StandardMacros.IncrementInt` (`self.triangleOffset`)))
      (if (`self.bCreatedMesh`)
        (`ProceduralMeshComponent.UpdateMeshSection_LinearColor` :`self` (`self.ProceduralMesh`) :`Vertices` (`self.Verts`) :`UV0` (`self.UVs`))
        (else
          (`ProceduralMeshComponent.CreateMeshSection_LinearColor` :`self` (`self.ProceduralMesh`) :`Vertices` (`self.Verts`) :`Triangles` (`self.Triangles`) :`UV0` (`self.UVs`))
          (`PrimitiveComponent.SetMaterial` (`self.ProceduralMesh`) 0 "/Game/TG/BP/test/m_lightsource.m_lightsource")
          (bind _returnvalue_4 (`PrimitiveComponent.CreateDynamicMaterialInstance` (`self.ProceduralMesh`) 0 "/Game/TG/BP/test/m_lightsource.m_lightsource" "None"))
          (`MaterialInstanceDynamic.SetVectorParameterValue` _returnvalue_4 "LightColor" (`self.lightColor`) :!label _label)
          (set `self.bCreatedMesh` true))))
    (:`then_1`
      (`KismetSystemLibrary.Delay` 1.0)
      (if (not (== (`self.lightColor`) (`self.originalColor`)))
        (`self.UpdateColor`)
        (set `self.originalColor` (`self.lightColor`))))))

(event `UpdateColor`
  (goto _label))

(fn `UserConstructionScript`
  (`SphereComponent.SetSphereRadius` (`self.LightSphereCollision`) (`self.LightDistance`) true))